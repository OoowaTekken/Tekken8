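; BP_PlayerCameraPawn is a test shared-camera pawn that follows the point between two BP_TESTCHARACTER players.
; On BeginPlay it finds all characters of that class, storing index zero as Player2 and any other as Player1.
; Each Tick it moves itself to their midpoint.
; Distance-based field of view and spring-arm length adjustments exist in the graph but are unconnected and never run.
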(event `self.ReceiveBeginPlay`
  (bind _outactors (`GameplayStatics.GetAllActorsOfClass` "/Game/LSJ/TEST/BP_TESTCHARACTER.BP_TESTCHARACTER_C"))
  (for (_array_element _array_index) _outactors
    (if (`KismetMathLibrary.Conv_IntToBool` _array_index)
      (set `self.Player1` _array_element)
      (else
        (set `self.Player2` _array_element)))))

(event `self.ReceiveTick`
  (params (DeltaSeconds :type "Float (single-precision)"))
  (bind _returnvalue (`self.K2_GetActorLocation` (`self.Player2`)))
  (`self.K2_SetActorLocation` (+ (* (- (`self.K2_GetActorLocation` (`self.Player1`)) _returnvalue) 0.5) _returnvalue)))

(fn `UserConstructionScript`)