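; Shared camera look-point actor that keeps a two-player view framed between Player1 and Player2.
; Each tick it first sets the MainCameraArm length to the distance between the two players, so the arm extends as they separate.
; It then moves itself to the midpoint of their locations without sweeping, with no smoothing or length clamping in the graph.
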(event `self.ReceiveBeginPlay`)

(event `self.ReceiveTick`
  (params (DeltaSeconds :type "Float (single-precision)"))
  (bind _returnvalue (`self.K2_GetActorLocation` (`self.Player2`)))
  (`|ExecutionSequence`
    (:`then_0`
      (`self.SetCameraLengh`))
    (:`then_1`
      (`self.K2_SetActorLocation` (+ _returnvalue (/ (- (`self.K2_GetActorLocation` (`self.Player1`)) _returnvalue) 2.0))))))

(event `SetCameraLengh`
  (set `SpringArmComponent.TargetArmLength` (* (`KismetMathLibrary.Abs` (`KismetMathLibrary.VSize` (- (`self.K2_GetActorLocation` (`self.Player1`)) (`self.K2_GetActorLocation` (`self.Player2`))))) 1.0) (`self.MainCameraArm`)))

(fn `UserConstructionScript`)